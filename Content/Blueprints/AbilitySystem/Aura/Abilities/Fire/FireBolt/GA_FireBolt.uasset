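; Fire Bolt gameplay ability that casts a projectile toward the point under the mouse.
; Target data under the mouse supplies the location, and the avatar turns to face it through the combat interface.
; It plays the cast montage and waits for its Fire Bolt gameplay event, then spawns the projectile at that target and ends the ability.
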(event Ability|EventActivateAbility
  (bind _datahandle (|TargetDataUnderMouse)
    (:ValidData
      (bind _output_get (Variables|Default|SetProjectileLocation (.Location (Collision|BreakHitResult (Ability|TargetData|GetHitResultfromTargetData _datahandle)))))
      (bind _ascombat_interface (Utilities|Casting|CastToCombatInterface (Ability|GetAvatarActorfromActorInfo)))
      (Class|CombatInterface|UpdateFacingTarget _ascombat_interface (Variables|Default|GetProjectileLocation))
      (|PlayMontageandWaitProxy "None" "/Game/Assets/Characters/Aura/Animations/Abilities/AM_FireBolt.AM_FireBolt" 1.0 "None" true 1.0 0.0
        (:then
          _)
        (:OnCompleted
          _))
      (Ability|Tasks|WaitGameplayEvent "(TagName=\"Event.Montage.FireBolt\")" 0
        (:EventReceived
          (Class|AuraProjectileSpell|SpawnProjectile (Variables|Default|GetProjectileLocation))
          (Ability|EndAbility))))))

(event Ability|EventOnEndAbility
  (params (bWasCancelled :type Boolean)))