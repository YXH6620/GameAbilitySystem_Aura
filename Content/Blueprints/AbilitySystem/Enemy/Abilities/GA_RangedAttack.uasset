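; Enemy gameplay ability for a ranged attack, currently a stub that only visualizes the attack origin and spawns no projectile.
; On activation it turns the avatar toward its combat target via interface messages and plays a random tagged attack montage.
; The montage's tag drives a gameplay event wait, then selects the combat socket location where a debug sphere is drawn.
; The graph never calls EndAbility.
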(event Ability|EventActivateAbility
  (bind _returnvalue (Ability|GetAvatarActorfromActorInfo))
  (bind _returnvalue_2 (Class|EnemyInterface|GetCombatTarget(Message) _returnvalue))
  (Class|CombatInterface|UpdateFacingTarget(Message) _returnvalue (Transformation|GetActorLocation _returnvalue_2))
  (bind _returnvalue_3 (Class|CombatInterface|GetAttackMontages(Message) (Ability|GetAvatarActorfromActorInfo)))
  (bind _output_get (Variables|Default|SetTagged%20Montage (Class|AuraDamageGameplayAbility|GetRandomTaggedMontage _returnvalue_3)))
  (|PlayMontageandWaitProxy "None" (.Montage (Utilities|Struct|BreakTaggedMontage _output_get)) 1.0 "None" false 1.0 0.0
    (:then
      (Ability|Tasks|WaitGameplayEvent (.MontageTag (Utilities|Struct|BreakTaggedMontage _output_get)) 0
        (:EventReceived
          (bind _returnvalue_4 (Class|CombatInterface|GetCombatSocketLocation(Message) (Ability|GetAvatarActorfromActorInfo) (.MontageTag (Utilities|Struct|BreakTaggedMontage _output_get))))
          (Rendering|Debug|DrawDebugSphere _returnvalue_4 5e+01 12 "(R=0.777955,G=0.011239,B=1.000000,A=1.000000)" 3.0))))))

(event Ability|EventOnEndAbility
  (params (bWasCancelled :type Boolean)))